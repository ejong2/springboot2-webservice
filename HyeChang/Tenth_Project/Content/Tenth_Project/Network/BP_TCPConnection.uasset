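; TCP client Blueprint that connects to a server at BeginPlay, tracks the connection ID and disconnects when destroyed.
; Received bytes are parsed into a four-integer header (message ID, size, sender, receiver), then dispatched by ID to S2C handlers, which are empty stubs.
; C2S functions build a matching header by concatenating bytes and send it without any payload, though nothing in this graph calls them.
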(event `self.ReceiveBeginPlay`
  (`self.NetConnecting`))

(event `self.ReceiveDestroyed`
  (`self.Disconnect` (`self.NetConnectionID`)))

(fn `C2S_ProcessPacket_1`
  (returns (Success :type Boolean))
  (if true
    (bind _outbytearray (`self.MakeMessageHeaderByteArray` 11001 (`self.In Message Size`) (`self.ClientSocketID`) (`self.ServerSocketID`)))
    (bind _returnvalue (`self.SendData` (`self.NetConnectionID`) _outbytearray))
    (if _returnvalue
      (return true)
      (else
        (return false)))))

(fn `C2S_ProcessPacket_2`
  (params (Byte :type Byte))
  (returns (Success :type Boolean))
  (if true
    (bind _outbytearray (`self.MakeMessageHeaderByteArray` 11002 (`self.In Message Size`) (`self.ClientSocketID`) (`self.ServerSocketID`)))
    (bind _returnvalue (`self.SendData` (`self.NetConnectionID`) _outbytearray))
    (if _returnvalue
      (return true)
      (else
        (return false)))))

(fn `C2S_ProcessPacket_3`
  (params (Byte :type Byte))
  (returns (Success :type Boolean))
  (if true
    (bind _outbytearray (`self.MakeMessageHeaderByteArray` 11003 (`self.In Message Size`) (`self.ClientSocketID`) (`self.ServerSocketID`)))
    (bind _returnvalue (`self.SendData` (`self.NetConnectionID`) _outbytearray))
    (if _returnvalue
      (return true)
      (else
        (return false)))))

(fn `C2S_ProcessPacket_4`
  (params (Byte :type Byte))
  (returns (Success :type Boolean))
  (if true
    (bind _outbytearray (`self.MakeMessageHeaderByteArray` 11004 (`self.In Message Size`) (`self.ClientSocketID`) (`self.ServerSocketID`)))
    (bind _returnvalue (`self.SendData` (`self.NetConnectionID`) _outbytearray))
    (if _returnvalue
      (return true)
      (else
        (return false)))))

(fn `GetMessageHeader`
  (params (InByteArray :type "Array of Byte"))
  (returns (OutByteArray :type "Array of Byte") (OutMessageHeader :type "/Game/Tenth_Project/Network/ST_MessageHeader Structure"))
  (bind _output_get (set `self.TempByteArray` InByteArray))
  (bind _returnvalue (`self.Message_ReadInt` _output_get))
  (bind _returnvalue_2 (`self.Message_ReadInt` _output_get))
  (bind _returnvalue_3 (`self.Message_ReadInt` _output_get))
  (bind _returnvalue_4 (`self.Message_ReadInt` _output_get))
  (return _output_get (make `/Game/Tenth_Project/Network/ST_MessageHeader` _returnvalue _returnvalue_2 _returnvalue_3 _returnvalue_4)))

(fn `MakeMessageHeaderByteArray`
  (params (InMessageID :type Integer) (InMessageSize :type Integer) (InSenderSocketID :type Integer) (InReceiverSocketID :type Integer))
  (returns (OutByteArray :type "Array of Byte"))
  (return (`self.Concat_BytesBytes` (`self.Conv_IntToBytes` InMessageID) (`self.Conv_IntToBytes` InMessageSize) (`self.Conv_IntToBytes` InSenderSocketID) (`self.Conv_IntToBytes` InReceiverSocketID))))

(fn `NetConnected`
  (params (ConnectionId :type Integer))
  (set `self.NetConnectionID` ConnectionId))

(fn `NetConnecting`
  (`self.Connect` (`self.Ip Address`) (`self.Port`) (`|CreateDelegate` :!event `NetDisconnectd`) (`|CreateDelegate` :!event `NetConnected`) (`|CreateDelegate` :!event `NetReceived`)))

(fn `NetDisconnectd`
  (params (ConnectionId :type Integer))
  (`self.Disconnect` ConnectionId)
  (set `self.NetConnectionID` -1))

(fn `NetProcessPacket`
  (params (ByteArray :type "Array of Byte"))
  (bind _output_get (set `self.TempByteArray` ByteArray))
  (if (>= (`KismetArrayLibrary.Array_Length` _output_get) 16)
    (bind (_outbytearray _outmessageheader) (`self.GetMessageHeader` (`self.TempByteArray`)))
    (set `self.TempByteArray` _outbytearray)
    (switch `int` (`.MessageID_8_F1FC1A2B4469523DC7D341B725E6FB44` (break `/Game/Tenth_Project/Network/ST_MessageHeader` _outmessageheader))
      (:`21001`
        (`self.S2C_ProcessPacket_1`))
      (:`21002`
        (`self.S2C_ProcessPacket_2`))
      (:`21003`
        (`self.S2C_ProcessPacket_3`))
      (:`21004`
        (`self.S2C_ProcessPacket_4`)))))

(fn `NetReceived`
  (params (ConnectionId :type Integer) (Message :type "Array of Byte (by ref)"))
  (set `self.NetConnectionID` ConnectionId)
  (bind _output_get (set `self.RecvBuffer` Message))
  (set `self.RecvLength` (`KismetArrayLibrary.Array_Length` Message))
  (`self.NetProcessPacket` _output_get)
  (return))

(fn `S2C_ProcessPacket_1`)

(fn `S2C_ProcessPacket_2`)

(fn `S2C_ProcessPacket_3`)

(fn `S2C_ProcessPacket_4`)

(fn `UserConstructionScript`)